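; Base player character for a 2D flipbook platformer, with multi-jump, dash, ammo-limited projectiles, health, lives and score.
; Tick picks the flipbook from velocity and turns the character via control rotation.
; Capsule hits on enemies use hit direction to either stomp-kill them or damage and knock back the player, gated by a resetting DoOnce.
; Stat changes update W_PlayerHUD; death drops the body off-screen, then respawns through BP_GameModeBase or shows game over.
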(event `self.ReceiveBeginPlay`
  (set `self.MovementState` "NewEnumerator4")
  ;[1 1 1] Create HUD widget, Update elements then display on screen.
  (bind _returnvalue (`|CreateWidget` "/Game/Blueprints/UserInterface/W_PlayerHUD.W_PlayerHUD_C"))
  (bind _output_get (set `self.PlayerHUDRef` _returnvalue))
  (`/Game/Blueprints/UserInterface/W_PlayerHUD.UpdateMessage` _output_get)
  (`self.Update Health`)
  (`self.Update Lives`)
  (`self.Update Ammo`)
  (`self.Update Score`)
  (`UserWidget.AddToViewport` _output_get 0)
  ;[1 1 1] Create Reference to GameModeBase
  (bind _asbp_game_mode_base (cast `/Game/Blueprints/BP_GameModeBase` (`GameplayStatics.GetGameMode`)))
  (set `self.GameModeBaseRef` _asbp_game_mode_base))

(event `self.ReceiveTick`
  (params (DeltaSeconds :type "Float (single-precision)"))
  (`|ExecutionSequence`
    (:`then_0`
      (`self.UpdateFlipBook`))
    (:`then_1`
      (`self.UpdatePlayerRotation`))))

(event `self.ReceiveAnyDamage`
  (params (Damage :type "Float (single-precision)") (DamageType :type "DamageType Object Reference") (InstigatedBy :type "Controller Object Reference") (DamageCauser :type "Actor Object Reference"))
  (bind _gamemodebaseref (`self.GameModeBaseRef`))
  (set `self.Health` (`KismetMathLibrary.FClamp` (- (`self.Health`) Damage) 0.0 (`self.Default Health`)))
  (`self.Update Health`)
  (if (and (<= (`self.Health`) 0.0) (not (`self.IsDead`)))
    (`self.Player Died`)
    ;[1 1 1] Check if Player has lives remaining
    (set `/Game/Blueprints/BP_GameModeBase.bIsTimerRunning` false _gamemodebaseref)
    (if (<= (`/Game/Blueprints/BP_GameModeBase.PlayerLives` _gamemodebaseref) 0)
      ;[1 1 1] If No Lives Remaining, show game over screen.
      (bind _returnvalue (`|CreateWidget` "/Game/Blueprints/UserInterface/W_GameOver.W_GameOver_C"))
      (`UserWidget.AddToViewport` _returnvalue 0)
      (else
        (`KismetSystemLibrary.Delay` 2.5)
        (bind _asbp_game_mode_base (cast `/Game/Blueprints/BP_GameModeBase` (`GameplayStatics.GetGameMode`)))
        (`/Game/Blueprints/BP_GameModeBase.PlayerRespawn` _asbp_game_mode_base)))
    (else
      ;[1 1 1] If the player takes damage and it doesn't kill them, play a sound.
      (`GameplayStatics.PlaySound2D` (`self.InjuredSFX`) 1.0 1.0 0.0 null null))))

(event `self.CapsuleComponent.OnComponentHit`
  (params (HitComponent :type "PrimitiveComponent Object Reference") (OtherActor :type "Actor Object Reference") (OtherComp :type "PrimitiveComponent Object Reference") (NormalImpulse :type "Vector Structure") (Hit :type "HitResult Structure (by ref)"))
  (bind (_hitdirection_x _hitdirection_y _hitdirection_z) (`KismetMathLibrary.BreakVector` (`self.HitDirection`)))
  (bind _hitenemyref (`self.HItEnemyRef`))
  (bind _hitdirection_x_2 (`KismetMathLibrary.BreakVector` (`self.HitDirection`)))
  (bind _asbp_enemy_base (cast `/Game/Blueprints/Enemies/BP_EnemyBase` OtherActor))
  (set `self.HItEnemyRef` _asbp_enemy_base)
  (`/Engine/EditorBlueprintResources/StandardMacros.DoOnce` false :!label _label
    (:`Completed`
      (set `self.HitDirection` (`KismetMathLibrary.Normal` (- Hit_Location (`self.K2_GetActorLocation`)) 0.0))
      (`|ExecutionSequence`
        (:`then_0`
          (if (<= _hitdirection_z -0.25)
            (set `self.JumpCount` 0)
            ;[1 1 1] damage enemy
            (`self.CancelMovement`)
            (`CharacterMovementComponent.AddImpulse` (`self.CharacterMovement`) (`KismetMathLibrary.MakeVector` 0.0 0.0 (`self.KnockBackForce`)) true) ; ticked velocity change, Z velocity to 500
            (`GameplayStatics.ApplyDamage` _hitenemyref (`/Game/Blueprints/Enemies/BP_EnemyBase.Health` _hitenemyref))
            (else
              ;[1 1 1] player damage
              (`self.CancelMovement`)
              (`CharacterMovementComponent.AddImpulse` (`self.CharacterMovement`) (`KismetMathLibrary.MakeVector` (* _hitdirection_x_2 (* -1.0 (`self.KnockBackForce`))) 0.0 (`self.KnockBackForce`)) true) ; ticked velocity change, Z velocity to 500
              (`GameplayStatics.ApplyDamage` self (`self.PlayerDamage`)))))
        (:`then_1`
          (`KismetSystemLibrary.Delay` 0.2)
          (`self.ResetHitCheck`))))))

(event `ResetHitCheck`
  (goto _label :!via `Reset`))

(event `InputAction|RangedAttack`
  (params (Key :type "Key Structure"))
  (:`Pressed`
    ;[0.1412 1 0] Fire projectile with delay between shots
    (if (`self.bCanFire?`)
      (`self.FireProjectile`)
      (`KismetSystemLibrary.Delay` (`self.DelayBetweenProjectiles`))
      (set `self.bCanFire?` true))))

(event `InputAxis|MoveRight`
  (params (AxisValue :type "Float (single-precision)"))
  ;[1 1 1] directional movement
  (`self.AddMovementInput` (1.0 0.0 0.0) AxisValue))

(event `InputAction|Jump`
  (params (Key :type "Key Structure"))
  ;[0.1406 1 0] Jumping
  (:`Pressed`
    ;;[1 1 1] Check if Jump is less than Max
    (if (< (`self.JumpCount`) (`self.MaxJumpCount`))
      ;;[1 1 1] If Character is in the air
      (if (`NavMovementComponent.IsFalling` (`self.CharacterMovement`))
        ;;[1 1 1] Air - Ninja Jump, Ground - Jump
        (`self.NinjaJump`)
        (else
          (`self.Jump`)
          ;;[1 1 1] Increase Jump Count
          (bind _result (`/Engine/EditorBlueprintResources/StandardMacros.IncrementInt` (`self.JumpCount`))
            (:`  `
              (set `self.JumpCount` _result))))))))

(event `self.OnLanded`
  (params (Hit :type "HitResult Structure (by ref)"))
  ;[0.1406 1 0] Jumping
  ;;[1 1 1] When player lands reset Jump count
  (set `self.JumpCount` 0))

(event `InputAction|Roll`
  (params (Key :type "Key Structure"))
  (:`Pressed`
    (`self.NinjaDash`)))

(event `NinjaDash`
  ;[1 1 1] Dash Function
  (if (`self.bCanDash?`)
    (set `self.bCanDash?` false)
    (if (`NavMovementComponent.IsFalling` (`self.CharacterMovement`))
      (`self.LaunchCharacter` (* (`self.GetActorForwardVector`) (`KismetMathLibrary.MakeVector` (`self.DashDistance`))))
      (`KismetSystemLibrary.Delay` 0.2)
      (set `MovementComponent.Velocity` (0.0 0.0 0.0) (`self.CharacterMovement`))
      (else
        (`self.LaunchCharacter` (* (`self.GetActorForwardVector`) (`KismetMathLibrary.MakeVector` (`self.DashDistance`))))))
    (`GameplayStatics.PlaySound2D` (`self.JumpSFX`) 1.0 1.0 0.0 null null)
    (`KismetSystemLibrary.Delay` 0.4)
    (set `self.bCanDash?` true)))

(fn `AddAmmo`
  (params (AmmoAmount :type Integer))
  (set `self.AmmoCount` (+ AmmoAmount (`self.AmmoCount`)))
  (`self.Update Ammo`))

(fn `AddHealth`
  (params (HealAmount :type "Float (double-precision)"))
  (set `self.Health` (`KismetMathLibrary.FClamp` (+ (`self.Health`) HealAmount) 0.0 (`self.Default Health`)))
  (`self.Update Health`))

(fn `AddScore`
  (params (ScoreValue :type Integer))
  (set `self.CurrentScore` (+ ScoreValue (`self.CurrentScore`)))
  (`self.Update Score`))

(fn `CancelMovement`
  (set `MovementComponent.Velocity` (0.0 0.0 0.0) (`self.CharacterMovement`))
  (`MovementComponent.StopMovementImmediately` (`self.CharacterMovement`))
  (`PrimitiveComponent.SetAllPhysicsLinearVelocity` (`self.CapsuleComponent`) (0.0 0.0 0.0) false))

(fn `FireProjectile`
  (bind _ammocount (`self.AmmoCount`))
  ;[1 1 1] Stops spamming
  (set `self.bCanFire?` false)
  ;[1 1 1] Checks  ammo
  (if (not (<= _ammocount 0))
    ;[1 1 1] Reduce ammo count by one and spawn projectile
    (bind _result (`/Engine/EditorBlueprintResources/StandardMacros.DecrementInt` _ammocount)
      (:`  `
        (bind _output_get (set `self.AmmoCount` _result))
        (`|SpawnActorFromClass` "/Game/Blueprints/Interactives/BP_PlayerProjectile.BP_PlayerProjectile_C" (`SceneComponent.K2_GetComponentToWorld` (`self.ProjectileSource`)) "Undefined" "MultiplyWithRoot" null null)
        ;[1 1 1] testing Sound
        (`GameplayStatics.PlaySound2D` "/Game/Audio_SoundEffects/Throwing.Throwing" 1.0 1.0 0.0 null null)
        ;[1 1 1] Update the HUD
        (`/Game/Blueprints/UserInterface/W_PlayerHUD.UpdateAmmo` (`self.PlayerHUDRef`) _output_get)
        (return)))))

(fn `NinjaJump`
  (bind (_x _y) (`KismetMathLibrary.BreakVector3f` (`self.GetVelocity`)))
  ;[1 1 1] Zero-out Z velocity for double jump
  (set `MovementComponent.Velocity` (`KismetMathLibrary.MakeVector` _x _y) (`self.CharacterMovement`))
  ;[1 1 1] Do Jump
  (`self.LaunchCharacter` (`GameplayStatics.GetPlayerCharacter` 0) (`KismetMathLibrary.MakeVector` 0.0 0.0 (`self.JumpHeight`)) false false)
  ;[1 1 1] Increase Jump Counter
  (bind _result (`/Engine/EditorBlueprintResources/StandardMacros.IncrementInt` (`self.JumpCount`))
    (:`  `
      (set `self.JumpCount` _result)
      ;[1 1 1] Play the Jump sound effect
      (`GameplayStatics.PlaySound2D` (`self.JumpSFX`) 1.0 1.0 0.0 null null))))

(fn `NinjaRoll`
  (if (`NavMovementComponent.IsFalling` (`self.CharacterMovement`))
    (`self.LaunchCharacter` (* (`self.GetActorForwardVector`) (`KismetMathLibrary.MakeVector` (/ (`self.DashDistance`) 100.0))))
    (else
      (`self.LaunchCharacter` (* (`self.GetActorForwardVector`) (`KismetMathLibrary.MakeVector` (`self.DashDistance`))))))
  (`GameplayStatics.PlaySound2D` (`self.JumpSFX`) 1.0 1.0 0.0 null null))

(fn `Player Died`
  (set `self.IsDead` true)
  ;[1 1 1] Play the death sound effect, and then remove this component again once finished.
  (`GameplayStatics.SpawnSoundAttached` (`self.DeathSFX`) (`self.CapsuleComponent`) "None" (0.0 0.0 0.0) (struct) "KeepRelativeOffset" false 1.0 1.0 0.0 null null)
  ;[1 1 1] Stop Current Player Movement
  (`self.DisableInput` (`GameplayStatics.GetPlayerController` 0))
  (`self.CancelMovement`)
  ;[1 1 1] Reduce Number of lives remaining by 1
  (bind _asbp_game_mode_base (cast `/Game/Blueprints/BP_GameModeBase` (`GameplayStatics.GetGameMode`)))
  (bind _result (`/Engine/EditorBlueprintResources/StandardMacros.DecrementInt` (`/Game/Blueprints/BP_GameModeBase.PlayerLives` _asbp_game_mode_base))
    (:`  `
      (set `/Game/Blueprints/BP_GameModeBase.PlayerLives` _result _asbp_game_mode_base)
      (`self.Update Lives`)
      ;[1 1 1] Death Effect (Pause Camera, Disable Collision, Make character bounce up and fall out of frame.
      (`SceneComponent.K2_DetachFromComponent` (`self.SpringArm`) "KeepWorld" "KeepRelative" "KeepRelative" true)
      (`PrimitiveComponent.SetCollisionResponseToAllChannels` (`self.CapsuleComponent`) "ECR_Ignore")
      (`PrimitiveComponent.SetSimulatePhysics` (`self.CapsuleComponent`) true)
      (`PrimitiveComponent.AddImpulse` (`self.CapsuleComponent`) (0.0 1.0 900.0) "None" true))))

(fn `Update Ammo`
  (`/Game/Blueprints/UserInterface/W_PlayerHUD.UpdateAmmo` (`self.PlayerHUDRef`) (`self.AmmoCount`)))

(fn `Update Health`
  (`/Game/Blueprints/UserInterface/W_PlayerHUD.UpdateHealth` (`self.PlayerHUDRef`) (`self.Health`) (`self.Default Health`)))

(fn `Update Lives`
  (bind _asbp_game_mode_base (cast `/Game/Blueprints/BP_GameModeBase` (`GameplayStatics.GetGameMode`)))
  (`/Game/Blueprints/UserInterface/W_PlayerHUD.UpdateLives` (`self.PlayerHUDRef`) (`/Game/Blueprints/BP_GameModeBase.PlayerLives` _asbp_game_mode_base)))

(fn `Update Score`
  (bind _asw_player_hud (cast `/Game/Blueprints/UserInterface/W_PlayerHUD` (`self.PlayerHUDRef`)))
  (`/Game/Blueprints/UserInterface/W_PlayerHUD.StoreGamemodeRef` _asw_player_hud)
  (`/Game/Blueprints/UserInterface/W_PlayerHUD.UpdateScore` (`self.PlayerHUDRef`) (`self.CurrentScore`)))

(fn `UpdateFlipBook`
  (bind (_returnvalue_x _returnvalue_y _returnvalue_z) (`KismetMathLibrary.BreakVector` (`self.GetVelocity`)))
  (set `self.MovementState` (select `bool` (!= (`KismetMathLibrary.VSize` (`self.GetVelocity`)) 0.0) :`false` "NewEnumerator0" :`true` (select `bool` (`NavMovementComponent.IsFalling` (`self.CharacterMovement`)) :`false` "NewEnumerator1" :`true` (select `bool` (<= _returnvalue_z 0.0) :`false` "NewEnumerator2" :`true` "NewEnumerator3" :!type "/Game/Blueprints/EPlayerMovement Enum"))))
  (`PaperFlipbookComponent.SetFlipbook` (`self.Sprite`) (select `/Game/Blueprints/EPlayerMovement` (`self.MovementState`) :`NewEnumerator0` (`self.FB_Idle`) :`NewEnumerator1` (`self.FB_Run`) :`NewEnumerator2` (`self.FB_Jump`) :`NewEnumerator3` (`self.FB_Fall`) :`NewEnumerator5` (`self.FB_Roll`))))

(fn `UpdatePlayerRotation`
  (bind _returnvalue_x (`KismetMathLibrary.BreakVector` (`self.GetVelocity`)))
  (`/Engine/EditorBlueprintResources/StandardMacros.CompareFloat` _returnvalue_x ; set up rotation
    (:`>`
      (`Controller.SetControlRotation` (`GameplayStatics.GetPlayerController` 0) (`KismetMathLibrary.MakeRotator` 0.0)) ; Move Right
    )
    (:`<`
      (`Controller.SetControlRotation` (`GameplayStatics.GetPlayerController` 0) (`KismetMathLibrary.MakeRotator` 0.0 0.0 180.0)) ; Move Left
    )))

(fn `UserConstructionScript`
  (set `self.Health` (`self.Default Health`)))
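; Base enemy Blueprint that handles taking damage and dying.
; AnyDamage subtracts damage from Health, clamped between zero and DefaultHealth, and uses an IsDead flag so death triggers only once.
; EnemyDied spawns the death sound at the capsule's location so it outlives the actor, then destroys the enemy.
; The construction script only assigns DefaultHealth to itself, so Health is not initialized in these graphs.
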(event `self.ReceiveAnyDamage`
  (params (Damage :type "Float (single-precision)") (DamageType :type "DamageType Object Reference") (InstigatedBy :type "Controller Object Reference") (DamageCauser :type "Actor Object Reference"))
  (set `self.Health` (`KismetMathLibrary.FClamp` (- (`self.Health`) Damage) 0.0 (`self.Default Health`)))
  (if (and (<= (`self.Health`) 0.0) (not (`self.IsDead`)))
    (set `self.IsDead` true)
    (`self.EnemyDied`)))

(fn `EnemyDied`
  ;[1 1 1] Spawn a sound effect at the location that the enemy is killed.  This avoids the sound getting cut off when the enemy actor is destroyed.
  (`GameplayStatics.SpawnSoundAtLocation` (`self.DeathSFX`) (`SceneComponent.K2_GetComponentLocation` (`self.CapsuleComponent`)) (struct) 1.0 1.0 0.0 null null)
  (`self.K2_DestroyActor`))

(fn `UserConstructionScript`
  (set `self.Default Health` (`self.Default Health`)))
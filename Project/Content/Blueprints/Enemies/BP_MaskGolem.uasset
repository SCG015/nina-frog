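; BP_MaskGolem is a side-scrolling enemy that patrols along the X axis, starting in a random direction and walking continuously through movement input each tick.
; When its capsule hits something other than the player with a horizontal normal, it reverses direction and mirrors its sprite by negating the X scale.
; A DoOnce gate that resets after a short delay debounces the turn.
; On death, it destroys itself after calling the parent handler.
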(event `self.ReceiveBeginPlay`
  (`parent.ReceiveBeginPlay`)
  (set `self.MoveRIght` (`KismetMathLibrary.RandomBool`))
  (`self.ToggleFacingDirection`))

(event `self.ReceiveTick`
  (params (DeltaSeconds :type "Float (single-precision)"))
  (`parent.ReceiveTick` DeltaSeconds)
  (`self.AddMovementInput` (1.0 0.0 0.0) (select `bool` (`self.MoveRIght`) :`false` -1.0 :`true` 1.0 :!type "Float (single-precision)")))

(event `self.CapsuleComponent.OnComponentHit`
  (params (HitComponent :type "PrimitiveComponent Object Reference") (OtherActor :type "Actor Object Reference") (OtherComp :type "PrimitiveComponent Object Reference") (NormalImpulse :type "Vector Structure") (Hit :type "HitResult Structure (by ref)"))
  (if (!= OtherActor (`GameplayStatics.GetPlayerPawn` 0))
    (if (!= (.x Hit_Normal) 0.0)
      (`/Engine/EditorBlueprintResources/StandardMacros.DoOnce` false :!label _label
        (:`Completed`
          (set `self.MoveRIght` (not (`self.MoveRIght`)))
          (`self.ToggleFacingDirection`)
          (`KismetSystemLibrary.Delay` 0.2)
          (`self.ResetDirectionChangeCheck`))))))

(event `ResetDirectionChangeCheck`
  (goto _label :!via `Reset`))

(fn `EnemyDied`
  (`parent.EnemyDied`)
  (`self.K2_DestroyActor`))

(fn `ToggleFacingDirection`
  (bind (_returnvalue_x _returnvalue_y _returnvalue_z) (`KismetMathLibrary.BreakVector` (`SceneComponent.K2_GetComponentScale` (`self.Sprite`))))
  (`SceneComponent.SetWorldScale3D` (`self.Sprite`) (`KismetMathLibrary.MakeVector` (* (`KismetMathLibrary.Abs` _returnvalue_x) (select `bool` (`self.MoveRIght`) :`false` 1.0 :`true` -1.0)) _returnvalue_y _returnvalue_z)))

(fn `UserConstructionScript`
  (`parent.UserConstructionScript`))
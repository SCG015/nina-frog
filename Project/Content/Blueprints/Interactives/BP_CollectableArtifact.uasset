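; BP_CollectableArtifact is an interactive pickup that awards score to the player who collects it.
; Its Interact override calls the parent, adds ScoreValue to the player, plays InteractSFX at the artifact's location with raised volume and pitch, then destroys the actor.
; The event graph holds only disabled default events, and the construction script just calls its parent.
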(fn `Interact`
  (params (PlayerRef :type "/Game/Blueprints/BP_PlayerBase Object Reference"))
  (`parent.Interact` PlayerRef)
  (`/Game/Blueprints/BP_PlayerBase.AddScore` (`local.PlayerRef`) (`self.ScoreValue`))
  (`GameplayStatics.SpawnSoundAtLocation` (`self.InteractSFX`) (`SceneComponent.K2_GetComponentLocation` (`self.Scene`)) (struct) 2.0 1.5 0.0 null null)
  (`self.K2_DestroyActor`))

(fn `UserConstructionScript`
  (`parent.UserConstructionScript`))
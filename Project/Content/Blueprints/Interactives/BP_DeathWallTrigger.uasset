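; Placed trigger that starts a death wall chase when the player pawn overlaps it.
; It spawns BP_DeathWall offset back along world X from the trigger, using preset Y and Z values.
; It then hides itself and disables collision on its box, flipbook and temporary placeholder.
; A W_DeathWall "RUN!" widget plays its opacity animation and is removed after that animation's length.
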(event `self.ReceiveActorBeginOverlap`
  (params (OtherActor :type "Actor Object Reference"))
  (bind _returnvalue (`self.GetTransform`))
  (bind _output_get (set `self.Other Actor` OtherActor))
  (if (== _output_get (`GameplayStatics.GetPlayerPawn` 0))
    ;[1 1 1] Spawn the death wall actor left of the position that the trigger has been placed
    (`|SpawnActorFromClass` "/Game/Blueprints/Enemies/BP_DeathWall.BP_DeathWall_C" (`KismetMathLibrary.MakeTransform` (`KismetMathLibrary.MakeVector` (- (.x (.location _returnvalue)) (`self.XOffset`)) (`self.YOffset`) (`self.ZWorld`)) (.rotation _returnvalue) (.scale _returnvalue)) "Undefined" "MultiplyWithRoot" null null)
    ;[1 1 1] Hide & Disable the trigger upon touch
    (`SceneComponent.SetHiddenInGame` (`self.Scene`) true true)
    (`PrimitiveComponent.SetCollisionEnabled` (`self.BoxInactivecollider`) "NoCollision")
    (`PrimitiveComponent.SetCollisionEnabled` (`self.PaperFlipbook`) "NoCollision")
    ;[1 0 0] DELETE WHEN FLIPBOOK ADDED
    (`PrimitiveComponent.SetCollisionEnabled` (`self.Placeholder-DeleteWhenFlipbookAdded`) "NoCollision")
    ;[1 1 1] Display the RUN! message on screen
    (bind _returnvalue_2 (`|CreateWidget` "/Game/Blueprints/UserInterface/W_DeathWall.W_DeathWall_C"))
    (`UserWidget.AddToViewport` _returnvalue_2 0)
    (bind _messageopacity (`/Game/Blueprints/UserInterface/W_DeathWall.MessageOpacity` _returnvalue_2))
    (bind _aswidget_animation (cast `WidgetAnimation` _messageopacity))
    (`UserWidget.PlayAnimation` _returnvalue_2 _aswidget_animation 0.0 1 "Forward" 1.0 false)
    (`KismetSystemLibrary.Delay` (`WidgetAnimation.GetEndTime` _messageopacity))
    (`Widget.RemoveFromParent` _returnvalue_2)
    (`parent.ReceiveActorBeginOverlap` (`self.Other Actor`))))

(fn `UserConstructionScript`
  (`parent.UserConstructionScript`))
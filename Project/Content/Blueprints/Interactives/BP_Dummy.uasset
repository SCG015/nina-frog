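; BP_Dummy is an interactive trigger that shows a hard-coded tutorial message about jump and movement controls on the player's HUD.
; When the player character enters its Box, it casts to BP_PlayerBase, sets the Message on PlayerHUDRef and calls UpdateMessage.
; Leaving the Box clears the message the same way, and both overlap events print debug strings, including when another actor overlaps.
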(event `self.Box.OnComponentBeginOverlap`
  (params (OverlappedComponent :type "PrimitiveComponent Object Reference") (OtherActor :type "Actor Object Reference") (OtherComp :type "PrimitiveComponent Object Reference") (OtherBodyIndex :type Integer) (bFromSweep :type Boolean) (SweepResult :type "HitResult Structure (by ref)"))
  (if (== OtherActor (`GameplayStatics.GetPlayerCharacter` 0))
    (`KismetSystemLibrary.PrintString` "player in range")
    (bind _asbp_player_base (cast `/Game/Blueprints/BP_PlayerBase` (`GameplayStatics.GetPlayerCharacter` 0)))
    (bind _playerhudref (`/Game/Blueprints/BP_PlayerBase.PlayerHUDRef` _asbp_player_base))
    (set `/Game/Blueprints/UserInterface/W_PlayerHUD.Message` "This is a tutorial message to help you. Space to jump, arrows to move." _playerhudref)
    (`/Game/Blueprints/UserInterface/W_PlayerHUD.UpdateMessage` _playerhudref)
    (else
      (`KismetSystemLibrary.PrintString` "it fucked up"))))

(event `self.Box.OnComponentEndOverlap`
  (params (OverlappedComponent :type "PrimitiveComponent Object Reference") (OtherActor :type "Actor Object Reference") (OtherComp :type "PrimitiveComponent Object Reference") (OtherBodyIndex :type Integer))
  (if (== OtherActor (`GameplayStatics.GetPlayerCharacter` 0))
    (`KismetSystemLibrary.PrintString` "player leaves range" true true (struct :`R` 0.0386 :`G` 1.0 :`B` 0.261365 :`A` 1.0))
    (bind _asbp_player_base (cast `/Game/Blueprints/BP_PlayerBase` (`GameplayStatics.GetPlayerCharacter` 0)))
    (bind _playerhudref (`/Game/Blueprints/BP_PlayerBase.PlayerHUDRef` _asbp_player_base))
    (set `/Game/Blueprints/UserInterface/W_PlayerHUD.Message` "" _playerhudref)
    (`/Game/Blueprints/UserInterface/W_PlayerHUD.UpdateMessage` _playerhudref)
    (else
      (`KismetSystemLibrary.PrintString` "IT FUCKED UP" true true (struct :`R` 0.0386 :`G` 1.0 :`B` 0.261365 :`A` 1.0)))))

(fn `UserConstructionScript`)
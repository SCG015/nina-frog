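; BP_EndGoal is the level exit that ends the level when the player pawn overlaps it.
; A one-shot overlap handler destroys all death walls, turns off tick and movement on every enemy, then disables player input and stops the player's momentum.
; After a short delay it shows the W_EndLevel widget with UI-only input and a visible cursor, rather than loading the next level automatically.
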(event `self.ReceiveActorBeginOverlap`
  (params (OtherActor :type "Actor Object Reference"))
  (bind _returnvalue (`GameplayStatics.GetPlayerController` 0))
  ;[1 1 1] Make sure that it's the player touching the exit.
  (if (== OtherActor (`GameplayStatics.GetPlayerPawn` 0))
    (`/Engine/EditorBlueprintResources/StandardMacros.DoOnce` false
      (:`Completed`
        ;[1 1 1] Remove and active death walls from play
        (bind _outactors (`GameplayStatics.GetAllActorsOfClass` "/Game/Blueprints/Enemies/BP_DeathWall.BP_DeathWall_C"))
        (for _array_element _outactors
          (`self.K2_DestroyActor` _array_element))
        ;[1 1 1] Stop all enemy activity
        (bind _outactors_2 (`GameplayStatics.GetAllActorsOfClass` "/Game/Blueprints/Enemies/BP_EnemyBase.BP_EnemyBase_C"))
        (for _array_element_2 _outactors_2
          (`self.SetActorTickEnabled` _array_element_2 false)
          (`MovementComponent.StopMovementImmediately` (`Character.CharacterMovement` _array_element_2)))
        ;[1 1 1] Stop Players from moving their character
        (`self.DisableInput` (`GameplayStatics.GetPlayerPawn` 0) (`GameplayStatics.GetPlayerController` 0))
        ;[1 1 1] Stop any existing momentum that would move them away from the exit
        (bind _asbp_player_base (cast `/Game/Blueprints/BP_PlayerBase` (`GameplayStatics.GetPlayerPawn` 0)))
        (`NavMovementComponent.StopMovementKeepPathing` (`Character.CharacterMovement` _asbp_player_base))
        (`KismetSystemLibrary.Delay` 1.0)
        ;[1 1 1] EndLevel widget added to goal instead of auto-next level
        (bind _returnvalue_2 (`|CreateWidget` "/Game/Blueprints/UserInterface/W_EndLevel.W_EndLevel_C" (`GameplayStatics.GetPlayerController` 0)))
        (`UserWidget.AddToViewport` _returnvalue_2 0)
        (`WidgetBlueprintLibrary.SetInputMode_UIOnlyEx` _returnvalue _returnvalue_2)
        (set `PlayerController.bShowMouseCursor` true _returnvalue)))))

(fn `UserConstructionScript`
  (`parent.UserConstructionScript`))
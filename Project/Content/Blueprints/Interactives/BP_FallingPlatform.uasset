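; Falling platform interactive for a Paper2D game that breaks away after the player touches it.
; The flipbook starts stopped; when the player pawn overlaps the inactive collider box, it calls Interact for sound and plays the animation from the start.
; After a delay equal to the flipbook length, the actor destroys itself.
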(event `self.ReceiveBeginPlay`
  (`parent.ReceiveBeginPlay`)
  (`PaperFlipbookComponent.Stop` (`self.PaperFlipbook`)))

(event `self.BoxInactivecollider.OnComponentBeginOverlap`
  (params (OverlappedComponent :type "PrimitiveComponent Object Reference") (OtherActor :type "Actor Object Reference") (OtherComp :type "PrimitiveComponent Object Reference") (OtherBodyIndex :type Integer) (bFromSweep :type Boolean) (SweepResult :type "HitResult Structure (by ref)"))
  (bind _paperflipbook (`self.PaperFlipbook`))
  ;[1 1 1] Check if it's the player overlapping the platform
  (if (== OtherActor (`GameplayStatics.GetPlayerPawn` 0))
    ;[1 1 1] Play Sound
    (`self.Interact` null)
    ;[1 1 1] Play Flipbook Animation
    (`PaperFlipbookComponent.PlayFromStart` _paperflipbook)
    ;[1 1 1] Wait until Flipbook Animation Ends
    (`KismetSystemLibrary.Delay` (`PaperFlipbookComponent.GetFlipbookLength` _paperflipbook))
    ;[1 1 1] Destroy Platform
    (`self.K2_DestroyActor`)))

(fn `UserConstructionScript`
  (`parent.UserConstructionScript`))
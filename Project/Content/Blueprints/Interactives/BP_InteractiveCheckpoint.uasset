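; BP_InteractiveCheckpoint is a checkpoint that updates the player's respawn point when touched.
; On overlap with the player pawn, it calls Interact with the BP_PlayerBase, writes its own transform to CurrentSpawn on BP_GameModeBase, then destroys itself.
; A flipbook swap meant to show a consumed checkpoint is left unconnected and never runs.
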(event `self.ReceiveActorBeginOverlap`
  (params (OtherActor :type "Actor Object Reference"))
  (bind _returnvalue (`GameplayStatics.GetPlayerPawn` 0))
  ;[1 1 1] Make sure it's the player touching the object
  (if (== OtherActor _returnvalue)
    (bind _asbp_player_base (cast `/Game/Blueprints/BP_PlayerBase` _returnvalue))
    (`self.Interact` _asbp_player_base)
    ;[1 1 1] Store the pawns new spawn location
    (bind _asbp_game_mode_base (cast `/Game/Blueprints/BP_GameModeBase` (`GameplayStatics.GetGameMode`)))
    (set `/Game/Blueprints/BP_GameModeBase.CurrentSpawn` (`self.GetTransform`) _asbp_game_mode_base)
    (`self.K2_DestroyActor`)))

(fn `UserConstructionScript`
  (`parent.UserConstructionScript`))
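; End-of-level goal that finishes the level when the player pawn overlaps its box collider.
; A DoOnce-gated overlap destroys every BP_DeathWall, then disables tick and stops movement on every BP_EnemyBase.
; After a short delay it shows the W_EndLevel widget, switching to UI-only input with a visible cursor.
; An older automatic jump to Level2 remains in the graph but never runs.
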(event `self.BoxInactivecollider.OnComponentBeginOverlap`
  (params (OverlappedComponent :type "PrimitiveComponent Object Reference") (OtherActor :type "Actor Object Reference") (OtherComp :type "PrimitiveComponent Object Reference") (OtherBodyIndex :type Integer) (bFromSweep :type Boolean) (SweepResult :type "HitResult Structure (by ref)"))
  (bind _returnvalue (`GameplayStatics.GetPlayerController` 0))
  (bind _output_get (set `self.Other Actor` OtherActor))
  (if (== _output_get (`GameplayStatics.GetPlayerPawn` 0))
    (`/Engine/EditorBlueprintResources/StandardMacros.DoOnce` false
      (:`Completed`
        (bind _outactors (`GameplayStatics.GetAllActorsOfClass` "/Game/Blueprints/Enemies/BP_DeathWall.BP_DeathWall_C"))
        (for _array_element _outactors
          (`self.K2_DestroyActor` _array_element))
        (bind _outactors_2 (`GameplayStatics.GetAllActorsOfClass` "/Game/Blueprints/Enemies/BP_EnemyBase.BP_EnemyBase_C"))
        (for _array_element_2 _outactors_2
          (`self.SetActorTickEnabled` _array_element_2 false)
          (`MovementComponent.StopMovementImmediately` (`Character.CharacterMovement` _array_element_2)))
        (`KismetSystemLibrary.Delay` 1.0)
        ;[1 1 1] EndLevel widget added to goal instead of auto-next level
        (bind _returnvalue_2 (`|CreateWidget` "/Game/Blueprints/UserInterface/W_EndLevel.W_EndLevel_C"))
        (`UserWidget.AddToViewport` _returnvalue_2 0)
        (`WidgetBlueprintLibrary.SetInputMode_UIOnlyEx` _returnvalue null)
        (set `PlayerController.bShowMouseCursor` true _returnvalue)))))

(fn `UserConstructionScript`
  (`parent.UserConstructionScript`))
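; BP_PlayerProjectile is the player's projectile, which kills enemies on contact and expires after a set lifetime.
; BeginPlay starts a timer of TimeAlive that destroys the projectile.
; On overlap with a BP_EnemyBase it applies Damage credited to its instigator, then destroys that enemy outright, whatever the damage amount, along with itself.
; Overlaps with other actors are ignored.
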(event `self.ReceiveBeginPlay`
  (`KismetSystemLibrary.K2_SetTimerDelegate` (delegate `OnTimeExpired`) (`self.TimeAlive`)))

(event `OnTimeExpired`
  (`self.K2_DestroyActor`))

(event `self.ReceiveActorBeginOverlap`
  (params (OtherActor :type "Actor Object Reference"))
  (bind _returnvalue (`self.GetInstigator`))
  (bind _asbp_enemy_base (cast `/Game/Blueprints/Enemies/BP_EnemyBase` OtherActor))
  (`GameplayStatics.ApplyDamage` _asbp_enemy_base (`self.Damage`) (`Pawn.GetController` _returnvalue) _returnvalue)
  (`self.K2_DestroyActor` _asbp_enemy_base)
  (`self.K2_DestroyActor`))

(fn `UserConstructionScript`)
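; BP_Spike is an interactive spike hazard that damages the player character on interaction.
; Its Interact override calls the parent logic, applies the spike damage value to the passed player reference, then restarts its Paper2D flipbook animation.
; A trailing DoOnce gates nothing, and the event graph holds only disabled placeholder events.
; An author note states that enemies are not hurt yet.
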(fn `Interact`
  (params (PlayerRef :type "/Game/Blueprints/BP_PlayerBase Object Reference"))
  ;[1 1 1] Currently only hurts the player character not enemies
  (`parent.Interact` PlayerRef)
  (`GameplayStatics.ApplyDamage` (`local.PlayerRef`) (`self.DamageValueSpike`))
  (`PaperFlipbookComponent.PlayFromStart` (`self.PaperFlipbook`))
  (`/Engine/EditorBlueprintResources/StandardMacros.DoOnce` false))

(fn `UserConstructionScript`
  (`parent.UserConstructionScript`))